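; BP_NPC is an interactable quest-giver that shows dialogue and gives the player a hard-coded "Take out the trash" task.
; Each Interact advances TalkIndex through the Dialogue array, showing the line in a W_Dialogue widget that is created once and reused.
; After the last line, it adds the task to BP_GameInstance's ActiveTasks, removes the widget and resets the index.
; ShowInfo sets the HUD's interaction prompt.
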(event `/Game/FirstPerson/Blueprints/BPI_Interactable.Interact`
  (bind _result (`/Engine/EditorBlueprintResources/StandardMacros.IncrementInt` (`self.talkIndex`))
    (:`  `
      (if (< _result (`KismetArrayLibrary.Array_Length` (`self.dialogue`)))
        (bind _dialogueui (`self.DialogueUI`)
          (:`then`
            (`UserWidget.AddToViewport` _dialogueui 0))
          (:`else`
            (bind _returnvalue (`|CreateWidget` "/Game/Quests/W_Dialogue.W_Dialogue_C" (`GameplayStatics.GetPlayerController` 0)))
            (bind _output_get (set `self.DialogueUI` _returnvalue))
            (`UserWidget.AddToViewport` _output_get 0)))
        (`TextBlock.SetText` (`/Game/Quests/W_Dialogue.dialogueText` (`self.DialogueUI`)) (`KismetTextLibrary.Conv_StringToText` (`|GetArrayItem` (`self.dialogue`) (`self.talkIndex`))))
        (else
          (bind _asbp_game_instance (cast `/Game/FirstPerson/Blueprints/BP_GameInstance` (`GameplayStatics.GetGameInstance`)))
          (`KismetArrayLibrary.Array_Add` (`/Game/FirstPerson/Blueprints/BP_GameInstance.ActiveTasks` _asbp_game_instance) "Take out the trash")
          (`Widget.RemoveFromParent` (`self.DialogueUI`))
          (set `self.talkIndex` -1))))))

(event `/Game/FirstPerson/Blueprints/BPI_Interactable.ShowInfo`
  (params (HUD :type "/Game/FirstPerson/Blueprints/WBP_AwakeHud Object Reference"))
  (`/Game/FirstPerson/Blueprints/WBP_AwakeHud.SetInfoText` HUD "Press [E] to hear request"))

(fn `UserConstructionScript`)